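; Rock obstacle that sets itself up as damageable with a small health pool and tumbles endlessly at random.
; BeginPlay stores the cube's current rotation, picks a random target and play rate, then a timeline lerps between them and restarts the cycle when finished.
; The lerp feeds axes out of order (roll from Z, pitch from X, yaw from Y), and parent BeginPlay fires on every timeline update.
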(event EventBeginPlay
  (bind _cube (Variables|Default|GetCube))
  (bind _relativerotation (Variables|/Script/Engine.SceneComponent|GetRelativeRotation _cube))
  ;[1 1 1] Random Rotation
  (bind _output_get (Variables|Default|SetMaxHealth 2e+01))
  (Variables|Default|SetCurrentHealth _output_get)
  (Variables|Default|SetbCanBeDamaged true)
  (|CurrentRotation (.roll _relativerotation) (.pitch _relativerotation) (.yaw _relativerotation) :!label _label)
  (|TargetRotation (Math|Random|RandomFloatinRange 0.0 3.6e+02) (Math|Random|RandomFloatinRange 0.0 3.6e+02) (Math|Random|RandomFloatinRange 0.0 3.6e+02))
  (Components|Timeline|SetPlayRate (Variables|Default|GetTimeline_0) (Math|Random|RandomFloatinRange 0.25 1.0))
  (bind _newtrack_0 (Timeline|Timeline_0 PlayFromStart)
    (:Update
      (Transformation|SetRelativeRotation (Variables|Default|GetCube) (Math|Rotator|MakeRotator (Math|Float|Lerp (Variables|Default|GetCurrentZ) (Variables|Default|GetTargetZ) _newtrack_0) (Math|Float|Lerp (Variables|Default|GetCurrentX) (Variables|Default|GetTargetX) _newtrack_0) (Math|Float|Lerp (Variables|Default|GetCurrentY) (Variables|Default|GetTargetY) _newtrack_0)) false false)
      (|CallParentFunction))
    (:Finished
      (goto _label))))

(event Collision|EventActorBeginOverlap
  (params (OtherActor :type Actor%20Object%20Reference))
  (|CallParentFunction OtherActor) ; This node is disabled and will not be called.\nDrag off pins to build functionality.
)

(event EventTick
  (params (DeltaSeconds :type Float%20%28single-precision%29))
  (|CallParentFunction DeltaSeconds) ; This node is disabled and will not be called.\nDrag off pins to build functionality.
)

(fn ConstructionScript
  (|CallParentFunction))