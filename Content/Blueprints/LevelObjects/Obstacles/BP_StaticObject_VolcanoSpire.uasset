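; Volcano spire obstacle that can be damaged and repeatedly erupts bursts of rocks.
; BeginPlay sets its health and starts a looping timer, then calls the parent.
; Each eruption waits a random delay, then spawns a random number of BP_VolcanoSpire_Rocks actors.
; Rocks appear around the Sphere component at an offset rotated by random upward-biased vectors, each with a random rotation and enlarged scale.
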(event Custom|SpawnVolcanoRocks
  (bind _returnvalue (Math|Random|RandomFloatinRange -3.6e+02 3.6e+02))
  (bind _returnvalue_2 (Math|Random|RandomFloatinRange -3.6e+02 3.6e+02))
  (bind _returnvalue_3 (Math|Vector|MakeVector _returnvalue_2 _returnvalue 45.0))
  (bind _returnvalue_4 (Math|Conversions|RotationFromXVector _returnvalue_3))
  ;[1 1 1] Spawn Rocks
  (Utilities|FlowControl|Delay (Math|Random|RandomFloatinRange 0.5 2.0))
  (for _index (range 0 (Math|Random|RandomIntegerinRange 5 11))
    (Game|SpawnActorfromClass "/Game/Blueprints/LevelObjects/Obstacles/BP_VolcanoSpire_Rocks.BP_VolcanoSpire_Rocks_C" (Math|Transform|MakeTransform (+ (Transformation|GetWorldLocation (Variables|Default|GetSphere)) (Math|Vector|RotateVector (Variables|Default|GetSpireOffset) _returnvalue_4)) _returnvalue_4 "2.000000,2.000000,2.000000") "AlwaysSpawn" 0 0)))

(event EventBeginPlay
  ;[1 1 1] Begin Play
  (bind _output_get (Variables|Default|SetMaxHealth 3e+01))
  (Variables|Default|SetCurrentHealth _output_get)
  (Variables|Default|SetbCanBeDamaged true)
  (Utilities|Time|SetTimerbyFunctionName 0 "SpawnVolcanoRocks" 1.0 true)
  (|CallParentFunction))

(event Collision|EventActorBeginOverlap
  (params (OtherActor :type Actor%20Object%20Reference))
  (|CallParentFunction OtherActor) ; This node is disabled and will not be called.\nDrag off pins to build functionality.
)

(event EventTick
  (params (DeltaSeconds :type Float%20%28single-precision%29))
  (|CallParentFunction DeltaSeconds) ; This node is disabled and will not be called.\nDrag off pins to build functionality.
)

(fn ConstructionScript
  (|CallParentFunction))