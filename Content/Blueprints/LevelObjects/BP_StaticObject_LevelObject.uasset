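; BP_StaticObject_LevelObject is a static level object with a mesh, a measured length and health values, set to be non-damageable.
; On BeginPlay it derives YLength from the mesh's local bounds, scaled by three and rotated -90 degrees around Z.
; It initializes health before calling the parent BeginPlay, then turns off CanBeDamaged afterward.
; Overlap and Tick are disabled stubs, and construction only calls the parent.
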(event EventBeginPlay
  (bind _staticmesh (Variables|Default|GetStaticMesh))
  (bind (_min _max) (Components|StaticMesh|GetLocalBounds _staticmesh))
  (Variables|Default|SetYLength (- (.x (Math|Vector|RotateVectorAroundAxis (* _max 3) -9e+01 "0, 0,1.000000")) (.x (Math|Vector|RotateVectorAroundAxis (* _min 3) -9e+01 "0, 0,1.000000"))))
  (bind _output_get (Variables|Default|SetMaxHealth 1e+02))
  (Variables|Default|SetCurrentHealth _output_get)
  (|CallParentFunction)
  (Variables|Default|SetbCanBeDamaged false))

(event Collision|EventActorBeginOverlap
  (params (OtherActor :type Actor%20Object%20Reference))
  (|CallParentFunction OtherActor) ; This node is disabled and will not be called.\nDrag off pins to build functionality.
)

(event EventTick
  (params (DeltaSeconds :type Float%20%28single-precision%29))
  (|CallParentFunction DeltaSeconds) ; This node is disabled and will not be called.\nDrag off pins to build functionality.
)

(fn ConstructionScript
  (|CallParentFunction))