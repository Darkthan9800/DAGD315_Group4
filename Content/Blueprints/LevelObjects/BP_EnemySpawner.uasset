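; Level spawner that places enemies and obstacles at random points within its collision component's bounds, at the actor's height.
; Looping timers drive both spawns through randomized Delays, with regular enemies capped by the game mode's enemy limit.
; Below that cap, every fifth kill also spawns a second enemy type, guarded by the last recorded kill count.
; The obstacle Delay sits inside a loop, so overlapping calls do not queue.
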(event Custom|SpawnEnemy
  (bind _bp_gamemode (Variables|Default|GetBP_GameMode))
  (bind _enemieskilled (Variables|/Game/Blueprints/BP_GameMode.BP_GameMode_C|GetEnemiesKilled _bp_gamemode))
  ;[1 1 1] Spawn Enemy 1
  (if (< (Variables|/Game/Blueprints/BP_GameMode.BP_GameMode_C|GetEnemyCount _bp_gamemode) (Variables|/Game/Blueprints/BP_GameMode.BP_GameMode_C|GetMaxEnemies _bp_gamemode))
    (if (and (== (Math|Integer|%(Integer) _enemieskilled 5) 0) (!= _enemieskilled (Variables|Default|GetCurrentEnemiesKilled)))
      (CallFunction|SpawnEnemy2))
    (Utilities|FlowControl|Delay (Math|Random|RandomFloatinRange 0.5 2.0))
    (Game|SpawnActorfromClass "/Game/Blueprints/LevelObjects/Enemies/BP_Enemy1.BP_Enemy1_C" (Math|Transform|MakeTransform (CallFunction|GetRandomLocation) "0, 0, 0" "1,1,1") "Undefined" 0 0)))

(event Custom|SpawnEnemy2
  ;[1 1 1] Spawning Enemy 2
  (Variables|Default|SetCurrentEnemiesKilled (Variables|/Game/Blueprints/BP_GameMode.BP_GameMode_C|GetEnemiesKilled (Variables|Default|GetBP_GameMode)))
  (Game|SpawnActorfromClass "/Game/Blueprints/LevelObjects/Enemies/BP_Enemy2.BP_Enemy2_C" (Math|Transform|MakeTransform (CallFunction|GetRandomLocation) "0, 0, 0" "1,1,1") "Undefined" 0 0))

(event Custom|SpawnObstacle
  ;[1 1 1] Obstacles
  (for _index (range 0 (Math|Random|RandomIntegerinRange 1 3))
    (Utilities|FlowControl|Delay (Math|Random|RandomFloatinRange 0.5 3.0))
    (Game|SpawnActorfromClass "/Game/Blueprints/LevelObjects/BP_StaticObject_Class.BP_StaticObject_Class_C" (Math|Transform|MakeTransform (CallFunction|GetRandomLocation) "0, 0, 0" "1,1,1") "Undefined" 0 0)))

(event EventBeginPlay
  ;[1 1 1] References and Variables
  (bind _asbp_game_mode (Utilities|Casting|CastToBP_GameMode (Game|GetGameMode)))
  (Variables|Default|SetBP_GameMode _asbp_game_mode)
  (Utilities|FlowControl|Sequence
    (:then_0
      (Utilities|Time|SetTimerbyFunctionName 0 "SpawnEnemy" 1.0 true))
    (:then_1
      (Utilities|Time|SetTimerbyFunctionName 0 "SpawnObstacle" 1.0 true))))

(fn ConstructionScript)

(fn GetRandomLocation
  (bind _collisioncomponent (Variables|Default|GetCollisionComponent))
  (bind (_origin _boxextent) (Collision|GetComponentBounds _collisioncomponent))
  (bind _returnvalue (Math|Random|RandomPointinBoundingBox _origin _boxextent))
  (return (Math|Vector|MakeVector (.x _returnvalue) (.y _returnvalue) (.z (Transformation|GetActorLocation)))))