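; BP_StaticObject_Class is a level object class that scrolls along negative Y at the game's level speed.
; BeginPlay caches the BP_GameMode reference.
; Tick then offsets the actor's location each frame by that game mode's LevelSpeed scaled by delta seconds, without sweep.
; An OnDespawnMessage call is present but never runs.
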(event EventBeginPlay
  ;[1 1 1] References and Variables
  (bind _asbp_game_mode (Utilities|Casting|CastToBP_GameMode (Game|GetGameMode)))
  (Variables|Default|SetBP_GameMode _asbp_game_mode))

(event Collision|EventActorBeginOverlap
  (params (OtherActor :type Actor%20Object%20Reference)))

(event EventTick
  (params (DeltaSeconds :type Float%20%28single-precision%29))
  ;[1 1 1] Movement
  (Transformation|SetActorLocation (+ (Transformation|GetActorLocation) (* (Math|Vector|MakeVector 0.0 (* (Variables|/Game/Blueprints/BP_GameMode.BP_GameMode_C|GetLevelSpeed (Variables|Default|GetBP_GameMode)) -1.0) 0.0) DeltaSeconds)) false false))

(fn ConstructionScript)