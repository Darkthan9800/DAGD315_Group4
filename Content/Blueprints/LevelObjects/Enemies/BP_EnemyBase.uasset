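; Base enemy actor that moves along negative world Y at a random speed and takes damage from bullets.
; On BeginPlay it registers with BP_GameMode's enemy count and caches the player character, whose BulletDamage sets each hit.
; Tick drives movement without sweep; the randomized MoveDirection is never read.
; Zero health updates count and kills before destruction, while BP_DespawnBox overlap destroys it without updating either.
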(event EventBeginPlay
  ;[1 1 1] References and Variables
  (Utilities|FlowControl|Sequence
    (:then_0
      (bind _asbp_game_mode (Utilities|Casting|CastToBP_GameMode (Game|GetGameMode)))
      (bind _output_get (Variables|Default|SetBP_GameMode _asbp_game_mode))
      (Default|UpdateEnemyCount _output_get 1)
      (Variables|Default|SetMoveDirection (Math|Random|RandomBool))
      (Variables|Default|SetMovementSpeed (Math|Random|RandomFloatinRange (Variables|Default|GetMinimumSpeed) (Variables|Default|GetMaximumSpeed)))
      (Variables|Default|SetSpawnLocation (Transformation|GetActorLocation))
      (Variables|Default|SetMoveEnabled true))
    (:then_1
      (bind _asbp_character (Utilities|Casting|CastToBP_Character (Game|Player|GetPlayerPawn 0))
        (:then
          (Variables|Default|SetBP_Character _asbp_character))
        (:CastFailed
          (Development|PrintString "failure"))))))

(event EventTick
  (params (DeltaSeconds :type Float%20%28single-precision%29))
  ;[1 1 1] Movement
  (if (Variables|Default|GetMoveEnabled)
    (Transformation|SetActorLocation (+ (Transformation|GetActorLocation) (* (Math|Vector|MakeVector 0.0 (* (Variables|Default|GetMovementSpeed) -1.0) 0.0) DeltaSeconds)) false false)))

(event Collision|EventActorBeginOverlap
  (params (OtherActor :type Actor%20Object%20Reference))
  (bind _returnvalue (Utilities|GetClass OtherActor))
  ;[1 1 1] Overlap
  (if (== _returnvalue "/Game/Blueprints/LevelObjects/BP_DespawnBox.BP_DespawnBox_C")
    (Actor|DestroyActor)
    (elif (== _returnvalue "/Game/Blueprints/PlayerCharacter/BP_Bullet.BP_Bullet_C")
      (CallFunction|DamageActor))))

(event EventDamageActor
  (bind _bp_gamemode (Variables|Default|GetBP_GameMode))
  ;[1 1 1] Damage Actor
  (Variables|Default|SetCurrentHealth (- (Variables|Default|GetCurrentHealth) (Variables|/Game/Blueprints/PlayerCharacter/BP_Character.BP_Character_C|GetBulletDamage (Variables|Default|GetBP_Character))))
  (if (<= (Variables|Default|GetCurrentHealth) 0.0)
    (Default|UpdateEnemyCount _bp_gamemode -1)
    (Default|UpdateEnemiesKilled _bp_gamemode 1)
    (Actor|DestroyActor)))

(fn ConstructionScript)